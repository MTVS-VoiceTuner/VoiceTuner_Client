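; Game manager for a music game that handles song selection and times a play session.
; Selecting a song creates the main UI with its image and title and passes the index to the BP_TrafficLight note spawner; cancelling resets that display.
; While playing, Tick accumulates time against hard-coded thresholds to start and end recording on the player character, then end the game.
; A separate stop event ends play early.
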(event Custom|CancleSong
  (Widget|SetVisibility (Variables|/Game/HSW/UI/WBP_MainUI.WBP_MainUI_C|GetCancelButton (Variables|Default|GetMainUI)) "Hidden")
  (Variables|Default|SetCurrentSong 0)
  (Appearance|SetBrushfromTexture (Variables|/Game/HSW/UI/WBP_MainUI.WBP_MainUI_C|GetCurrentSongImage (Variables|Default|GetMainUI)) "/Engine/EditorLandscapeResources/DefaultAlphaTexture.DefaultAlphaTexture" false)
  (Variables|/Script/UMG.TextBlock|SetText (Variables|/Game/HSW/UI/WBP_MainUI.WBP_MainUI_C|GetSongTitle (Variables|Default|GetMainUI)) "None"))

(event Custom|SetCurrentSong
  (params (CurrentSong :type Audio%20Component%20Object%20Reference) (Image :type Texture%202D%20Object%20Reference) (SingerSongName :type String) (Index :type Integer))
  (Variables|Default|SetCurrentSong CurrentSong)
  (bind _returnvalue (UserInterface|CreateWidget "/Game/HSW/UI/WBP_MainUI.WBP_MainUI_C"))
  (bind _output_get (Variables|Default|SetMainUI _returnvalue))
  (UserInterface|Viewport|AddtoViewport _output_get 0)
  (Appearance|SetBrushfromTexture (Variables|/Game/HSW/UI/WBP_MainUI.WBP_MainUI_C|GetCurrentSongImage (Variables|Default|GetMainUI)) Image false)
  (Variables|/Script/UMG.TextBlock|SetText (Variables|/Game/HSW/UI/WBP_MainUI.WBP_MainUI_C|GetSongTitle (Variables|Default|GetMainUI)) (Utilities|Text|ToText(String) SingerSongName))
  (Widget|SetVisibility (Variables|/Game/HSW/UI/WBP_MainUI.WBP_MainUI_C|GetCancelButton (Variables|Default|GetMainUI)) "Visible")
  (Default|SetMusic (Variables|Default|GetNoteSpawner) Index))

(event Custom|stop%20game
  (Variables|Default|SetIsPlaying false)
  (bind _asbp_hsw_third_person_character (Utilities|Casting|CastToBP_HSW_ThirdPersonCharacter (Game|Player|GetPlayerPawn 0)))
  (Default|GameEnd _asbp_hsw_third_person_character))

(event Collision|EventActorBeginOverlap
  (params (OtherActor :type Actor%20Object%20Reference)))

(event EventTick
  (params (DeltaSeconds :type Float%20%28single-precision%29))
  (if (Variables|Default|GetIsPlaying)
    (Variables|Default|SetPlayingTime (+ (Variables|Default|GetPlayingTime) DeltaSeconds))
    (if (Math|Boolean|ANDBoolean (>= (Variables|Default|GetPlayingTime) 81.5) (< (Variables|Default|GetPlayingTime) 104.0) (not (Variables|Default|GetRecordStart)))
      (Variables|Default|SetRecordStart true)
      (bind _asbp_hsw_third_person_character (Utilities|Casting|CastToBP_HSW_ThirdPersonCharacter (Game|Player|GetPlayerPawn 0)))
      (Default|RecordStart _asbp_hsw_third_person_character)
      (elif (and (>= (Variables|Default|GetPlayingTime) 106.5) (Variables|Default|GetRecordStart))
        (Variables|Default|SetRecordStart false)
        (bind _asbp_hsw_third_person_character_2 (Utilities|Casting|CastToBP_HSW_ThirdPersonCharacter (Game|Player|GetPlayerPawn 0)))
        (Default|RecordEnd _asbp_hsw_third_person_character_2)
        (elif (>= (Variables|Default|GetPlayingTime) 234.0)
          (Variables|Default|SetPlayingTime 0.0)
          (Variables|Default|SetIsPlaying false)
          (bind _asbp_hsw_third_person_character_3 (Utilities|Casting|CastToBP_HSW_ThirdPersonCharacter (Game|Player|GetPlayerPawn 0)))
          (Default|GameEnd _asbp_hsw_third_person_character_3))))))

(event EventBeginPlay
  (bind _returnvalue (Actor|GetActorOfClass "/Game/LDG/Blueprint/BP_TrafficLight.BP_TrafficLight_C"))
  (Variables|Default|SetNoteSpawner _returnvalue))

(fn ConstructionScript)