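; BPC_LightControl is a component that switches between default and in-game gobo lights in the level and triggers their hit effect.
; On BeginPlay it caches every BP_GoboLight and BP_DefaultGoboLight actor into two arrays.
; Custom events loop over those arrays to show or hide each set independently, or to call OnHitLight on every game gobo light.
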(event Custom|HitLight
  (for _array_element (Variables|Default|GetLights)
    (Default|OnHitLight _array_element)))

(event Custom|OnDefaultLight
  (for _array_element (Variables|Default|GetDefalutLights)
    (Rendering|SetActorHiddenInGame _array_element false)))

(event Custom|OffDefaultLight
  (for _array_element (Variables|Default|GetDefalutLights)
    (Rendering|SetActorHiddenInGame _array_element true)))

(event Custom|OnGameLight
  (for _array_element (Variables|Default|GetLights)
    (Rendering|SetActorHiddenInGame _array_element false)))

(event Custom|OffGameLight
  (for _array_element (Variables|Default|GetLights)
    (Rendering|SetActorHiddenInGame _array_element true)))

(event EventBeginPlay
  (bind _outactors (Actor|GetAllActorsOfClass "/Game/TA/Light/BP_GoboLight.BP_GoboLight_C"))
  (Variables|Default|SetLights _outactors)
  (bind _outactors_2 (Actor|GetAllActorsOfClass "/Game/TA/Light/BP_DefaultGoboLight.BP_DefaultGoboLight_C"))
  (Variables|Default|SetDefalutLights _outactors_2))

(event EventTick
  (params (DeltaSeconds :type Float%20%28single-precision%29)))