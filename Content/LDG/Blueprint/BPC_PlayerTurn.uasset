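; BPC_PlayerTurn is a turn component for BP_Guy02 players that indexes each one and cycles the current turn among them.
; A timer chain with per-step delays from a Time array advances CurrentTurn with modulo wraparound until the sequence runs out.
; Each change flip-flops the in-game widget's turn animation forward or reverse, setting Name from the game instance or a hardcoded string.
; The check for the player's own turn has no action attached.
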(event Custom|SwitchTurn
  ;[1 1 1] Switch Turn
  (CallFunction|Timer))

(event Custom|GetPlayers
  ;[1 1 1] Get Players
  (bind _outactors (Actor|GetAllActorsOfClass "/Game/TA/SubcultureGuy/Blueprints/BP_Guy02.BP_Guy02_C"))
  (bind _output_get (Variables|Default|SetPlayers _outactors))
  (for (_array_element _array_index) _output_get
    (Variables|BPC_PlayerTurn_C|SetTurn (Variables|/Game/HSW/ThirdPerson/Blueprints/BP_HSW_ThirdPersonCharacter.BP_HSW_ThirdPersonCharacter_C|GetBPC_PlayerTurn _array_element) _array_index)))

(event Custom|Timer
  ;[1 1 1] Switch Turn
  (Utilities|Time|SetTimerbyEvent (delegate Custom|ChangeTurn) (Utilities|Array|Get(acopy) (Variables|Default|GetTime) (Variables|Default|GetSequence))))

(event Custom|GetInGameWidget
  (params (NewParam :type WBP%20Mrchulyrics%20Object%20Reference))
  (bind _widgetanims (Variables|Default|GetWidgetAnims))
  ;[1 1 1] Switch Turn
  (bind _output_get (Variables|Default|SetInGameWidget NewParam))
  (Utilities|Array|Add _widgetanims (Variables|/Game/SHK/Blueprints/WBP_Mrchulyrics.WBP_Mrchulyrics_C|GetGetTurn_Player1 _output_get))
  (Utilities|Array|Add _widgetanims (Variables|/Game/SHK/Blueprints/WBP_Mrchulyrics.WBP_Mrchulyrics_C|GetGetTurn_Player2 _output_get)))

(event Custom|ChangeTurn
  (bind _sequence (Variables|Default|GetSequence))
  ;[1 1 1] Switch Turn
  (Utilities|FlowControl|Sequence
    (:then_0
      (bind _result (Math|Integer|IncrementInt (Variables|Default|GetCurrentTurn))
        (:%20%20
          (Variables|Default|SetCurrentTurn (Math|Integer|%(Integer) _result (Utilities|Array|Length (Variables|Default|GetPlayers))))
          (CallFunction|MyTurnWidgetAnim)
          (if (<= _sequence (Utilities|Array|Length (Variables|Default|GetTime)))
            (Math|Integer|IncrementInt _sequence
              (:%20%20
                (CallFunction|Timer)))))))
    (:then_1
      (if (== (Variables|Default|GetCurrentTurn) (Variables|Default|GetTurn))
        _))))

(event Custom|MyTurnWidgetAnim
  (bind _ingamewidget (Variables|Default|GetInGameWidget))
  (bind _widgetanims (Variables|Default|GetWidgetAnims))
  (bind _turn (Variables|Default|GetTurn))
  (bind _output (Utilities|Array|Get(acopy) _widgetanims _turn))
  ;[1 1 1] Switch Turn
  (Utilities|FlowControl|FlipFlop
    (:A
      (UserInterface|Animation|PlayAnimation _ingamewidget _output 0.0 1 "Forward" 1.0 false)
      (bind _asbp_hsw_game_instance (Utilities|Casting|CastToBP_HSW_GameInstance (Game|GetGameInstance)))
      (Variables|Default|SetName (Utilities|Text|ToText(String) (Class|HSWNetGameInstance|GetName _asbp_hsw_game_instance))))
    (:B
      (Class|UserWidget|PlayAnimationReverse _ingamewidget _output 1.0 false)
      (Variables|Default|SetName "메아미정은지"))))

(event EventBeginPlay)

(event EventTick
  (params (DeltaSeconds :type Float%20%28single-precision%29)))