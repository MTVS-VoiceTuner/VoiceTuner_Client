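; Playable singer character for a voice-controlled music minigame, with chair sitting and a toggleable list widget near BP_Front.
; Ready, GameStart and GameEnd handle positioning, music, UI and hit-tool visibility through world actors cached at BeginPlay.
; AudioCapture's envelope drives the hit tool's clamped height and enables its collision only above a loudness threshold.
; RecordStart and RecordEnd capture a submix to WAV, then trigger its upload via BP_HttpActor.
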(event OnComponentBeginOverlap(CapsuleComponent)
  (params (OverlappedComponent :type Primitive%20Component%20Object%20Reference) (OtherActor :type Actor%20Object%20Reference) (OtherComp :type Primitive%20Component%20Object%20Reference) (OtherBodyIndex :type Integer) (bFromSweep :type Boolean) (SweepResult :type Hit%20Result%20Structure%20%28by%20ref%29))
  ;[1 1 1] Overlap
  (bind _asbp_chair (Utilities|Casting|CastToBP_Chair OtherActor)
    (:then
      (Variables|Default|SetChair_0 _asbp_chair)
      (Variables|Default|SetCanSitting_0 true))
    (:CastFailed
      (Utilities|Casting|CastToBP_Front OtherActor)
      (bind _output_get (Variables|Default|SetCanViewList_0 true))
      (Development|PrintString (Utilities|String|ToString(Boolean) _output_get)))))

(event OnComponentEndOverlap(CapsuleComponent)
  (params (OverlappedComponent :type Primitive%20Component%20Object%20Reference) (OtherActor :type Actor%20Object%20Reference) (OtherComp :type Primitive%20Component%20Object%20Reference) (OtherBodyIndex :type Integer))
  ;[1 1 1] Overlap
  (bind _asbp_chair (Utilities|Casting|CastToBP_Chair OtherActor)
    (:then
      (Variables|Default|SetChair_0 _asbp_chair)
      (Variables|Default|SetCanSitting_0 false))
    (:CastFailed
      (Utilities|Casting|CastToBP_Front OtherActor)
      (bind _output_get (Variables|Default|SetCanViewList_0 false))
      (Development|PrintString (Utilities|String|ToString(Boolean) _output_get)))))

(event OnAudioEnvelopeValue(AudioCapture_0)
  (params (EnvelopeValue :type Float%20%28single-precision%29))
  (bind _minheight_0 (Variables|Default|GetMinHeight_0))
  (bind _hittool_0 (Variables|Default|GetHitTool_0))
  (bind _hittool_0_2 (Variables|Default|GetHitTool_0))
  (bind _maxheight_0 (Variables|Default|GetMaxHeight_0))
  (bind _returnvalue (Math|Float|MapRangeClamped EnvelopeValue 0.0 1.0 _minheight_0 _maxheight_0))
  (bind _returnvalue_2 (Transformation|GetActorLocation _hittool_0))
  (bind _hitcollision (Variables|/Script/VoiceTuner.HitTool|GetHitCollision _hittool_0_2))
  (bind _returnvalue_3 (+ (.z _returnvalue_2) _returnvalue))
  (if (>= _returnvalue_3 7e+02)
    (Variables|Default|SetElavateValue_0 7e+02)
    (elif (<= _returnvalue_3 4e+02)
      (Variables|Default|SetElavateValue_0 4e+02)
      (else
        (Variables|Default|SetElavateValue_0 _returnvalue_3))))
  (Transformation|SetWorldLocation (Variables|/Script/Engine.Actor|GetRootComponent (Variables|Default|GetHitTool_0)) (Math|Vector|MakeVector (.x _returnvalue_2) (.y _returnvalue_2) (Variables|Default|GetElavateValue_0)) false false)
  (if (> EnvelopeValue 0.03)
    (Collision|SetCollisionEnabled _hitcollision "QueryOnly")
    (else
      (Collision|SetCollisionEnabled _hitcollision "NoCollision"))))

(event OnComponentActivated(AudioCapture_0)
  (params (Component :type Actor%20Component%20Object%20Reference) (bReset :type Boolean)))

(event OnComponentDeactivated(AudioCapture_0)
  (params (Component :type Actor%20Component%20Object%20Reference)))

(event Custom|Sitting
  (bind _chair_0 (Variables|Default|GetChair_0))
  ;[1 1 1] 앉고 일어서는 세팅
  (Pawn|Components|CharacterMovement|SetMovementMode (Variables|Character|GetCharacterMovement) "MOVE_None" 0)
  (Transformation|SetActorLocationAndRotation (+ (Transformation|GetActorLocation _chair_0) "0.000000,0.000000,90.000000") (Transformation|GetActorRotation _chair_0))
  (Variables|/Script/Engine.SpringArmComponent|SetTargetArmLength (Variables|Default|GetCameraBoom) 2e+02))

(event Custom|UnSitting
  ;[1 1 1] 앉고 일어서는 세팅
  (Pawn|Components|CharacterMovement|SetMovementMode (Variables|Character|GetCharacterMovement) "MOVE_Walking" 0)
  (Variables|/Script/Engine.SpringArmComponent|SetTargetArmLength (Variables|Default|GetCameraBoom) 5e+02)
  (Transformation|SetRelativeLocation (Variables|Default|GetCameraBoom) "0.000000,0.000000,70.000000" false false))

(event Custom|Ready
  ;[1 1 1] 준비와 게임시작
  (Pawn|Components|CharacterMovement|SetMovementMode (Variables|Character|GetCharacterMovement) "MOVE_None" 0)
  (bind _returnvalue (Actor|GetActorOfClass "/Game/HSW/Blueprints/BP_SpawnPosition.BP_SpawnPosition_C"))
  (Transformation|SetActorLocationAndRotation (+ (Transformation|GetActorLocation _returnvalue) "0.000000,0.000000,70.000000") (Transformation|GetActorRotation _returnvalue)))

(event Custom|GameStart
  ;[1 1 1] 준비와 게임시작
  (Default|PlayMusic (Variables|Default|GetMusicBox_0))
  (Variables|/Game/HSW/Blueprints/BP_GameManager.BP_GameManager_C|SetIsPlaying (Variables|Default|GetGameManager_0) true)
  (Variables|/Script/Engine.PlayerController|SetbShowMouseCursor (Game|GetPlayerController 0) false)
  (Widget|SetVisibility (Variables|Default|GetGameUI_0) "Visible")
  (Components|Activation|SetActive (Variables|Default|GetAudioCapture_0) true false)
  (Rendering|SetActorHiddenInGame (Variables|Default|GetHitTool_0) false)
  (Rendering|SetActorHiddenInGame (Variables|Default|GetMusicBox_0) false))

(event Custom|UnDoReady
  ;[1 1 1] 준비와 게임시작
  (Pawn|Components|CharacterMovement|SetMovementMode (Variables|Character|GetCharacterMovement) "MOVE_Walking" 0))

(event Custom|RecordEnd
  (Audio|Components|Audio|Stop (Variables|Default|GetAudioCapture_0))
  (Class|AudioMixerBlueprintLibrary|StopRecordingOutput "WavFile" "Sinhodeong_CUT" "" "/Game/HSW/Resource/Sound/SSM_Record.SSM_Record" 0)
  (Class|HttpActor|SendSoundFiletoServer (Variables|Default|GetHttpActor_0)))

(event Custom|RecordStart
  (CameraShake|Start (Variables|Default|GetAudioCapture_0))
  (Class|AudioMixerBlueprintLibrary|StartRecordingOutput 0.0 "/Game/HSW/Resource/Sound/SSM_Record.SSM_Record"))

(event Custom|GameEnd
  ;[1 1 1] 준비와 게임시작
  (Default|StopMusic (Variables|Default|GetMusicBox_0))
  (Widget|SetVisibility (Variables|Default|GetGameUI_0) "Hidden")
  (Components|Activation|SetActive (Variables|Default|GetAudioCapture_0) true false)
  (Rendering|SetActorHiddenInGame (Variables|Default|GetHitTool_0) true)
  (Pawn|Components|CharacterMovement|SetMovementMode (Variables|Character|GetCharacterMovement) "MOVE_Walking" 0)
  (Rendering|SetActorHiddenInGame (Variables|Default|GetMusicBox_0) true))

(event EventBeginPlay
  (bind _returnvalue (UserInterface|CreateWidget "/Game/HSW/UI/WBP_HSWProtoFront.WBP_HSWProtoFront_C"))
  (bind _output_get (Variables|Default|SetFrontList_0 _returnvalue))
  (UserInterface|Viewport|AddtoViewport _output_get 0)
  (Widget|SetVisibility (Variables|Default|GetFrontList_0) "Hidden")
  (bind _returnvalue_2 (Actor|GetActorOfClass "/Game/LDG/Blueprint/BP_HitTool.BP_HitTool_C"))
  (Variables|Default|SetHitTool_0 _returnvalue_2)
  (bind _returnvalue_3 (Actor|GetActorOfClass "/Game/LDG/Blueprint/BP_TrafficLight.BP_TrafficLight_C"))
  (Variables|Default|SetMusicBox_0 _returnvalue_3)
  (bind _returnvalue_4 (Actor|GetActorOfClass "/Game/HSW/Blueprints/BP_GameManager.BP_GameManager_C"))
  (Variables|Default|SetGameManager_0 _returnvalue_4)
  (bind _returnvalue_5 (UserInterface|CreateWidget "/Game/LDG/UI/WBP_NoteWidget.WBP_NoteWidget_C"))
  (bind _output_get_2 (Variables|Default|SetGameUI_0 _returnvalue_5))
  (UserInterface|Viewport|AddtoViewport _output_get_2 0)
  (Widget|SetVisibility _output_get_2 "Hidden")
  (bind _returnvalue_6 (Actor|GetActorOfClass "/Game/SHK/Blueprints/BP_HttpActor.BP_HttpActor_C"))
  (Variables|Default|SetHttpActor_0 _returnvalue_6))

(event EventTick
  (params (DeltaSeconds :type Float%20%28single-precision%29)))

(event Input|KeyboardEvents|V
  (params (Key :type Key%20Structure :default "None")))

(event Input|KeyboardEvents|C
  (params (Key :type Key%20Structure :default "None"))
  (bind _frontlist_0 (Variables|Default|GetFrontList_0))
  ;[1 1 1] C키 바인딩(앉기, 일어서기)
  (:Pressed
    (Utilities|FlowControl|Sequence
      (:then_0
        (if (Variables|Default|GetIsSitting_0)
          (Variables|Default|SetIsSitting_0 false)
          (CallFunction|UnSitting)
          (elif (Variables|Default|GetCanSitting_0)
            (Variables|Default|SetIsSitting_0 true)
            (CallFunction|Sitting))))
      (:then_1
        (if (Variables|Default|GetCanViewList_0)
          (Utilities|FlowControl|FlipFlop
            (:A
              (Widget|SetVisibility _frontlist_0 "Visible"))
            (:B
              (Widget|SetVisibility _frontlist_0 "Hidden"))))))))

(event Input|KeyboardEvents|1
  (params (Key :type Key%20Structure :default "None")))

(event Input|KeyboardEvents|R
  (params (Key :type Key%20Structure :default "None"))
  (:Pressed
    (Default|StopGame (Variables|Default|GetGameManager_0))))

(fn ConstructionScript)