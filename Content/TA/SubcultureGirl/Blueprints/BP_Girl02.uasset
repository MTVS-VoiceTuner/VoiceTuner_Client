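; BP_Girl02 is a modular character Blueprint that assembles a girl from separate skeletal mesh parts for outfit and body.
; Its construction script sets the main Mesh as leader pose for the jacket, boots, socks, skirt, arms, lower body, bracers and glove, so they follow its animation.
; The SKHairA component is left out of the leader pose binding.
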(fn ConstructionScript
  (Components|SkinnedMesh|SetLeaderPoseComponent (Variables|Default|GetSK_BikerJacketA) (Variables|Character|GetMesh) false false))